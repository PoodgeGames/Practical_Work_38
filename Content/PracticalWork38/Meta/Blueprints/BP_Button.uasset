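; BP_Button is an interactable button actor that keeps an on/off state and broadcasts changes to it.
; Box overlap events set an InBox flag while a BP_ThirdPersonCharacter is inside the trigger.
; Separate Lighton and LightOff events set IsOn and fire the OnPressed dispatcher with the new value.
; Nothing in this graph reads InBox or calls those two events.
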(event `self.Box.OnComponentBeginOverlap`
  (params (OverlappedComponent :type "PrimitiveComponent Object Reference") (OtherActor :type "Actor Object Reference") (OtherComp :type "PrimitiveComponent Object Reference") (OtherBodyIndex :type Integer) (bFromSweep :type Boolean) (SweepResult :type "HitResult Structure (by ref)"))
  (cast `/Game/ThirdPerson/Blueprints/BP_ThirdPersonCharacter` OtherActor)
  (set `self.InBox` true))

(event `self.Box.OnComponentEndOverlap`
  (params (OverlappedComponent :type "PrimitiveComponent Object Reference") (OtherActor :type "Actor Object Reference") (OtherComp :type "PrimitiveComponent Object Reference") (OtherBodyIndex :type Integer))
  (cast `/Game/ThirdPerson/Blueprints/BP_ThirdPersonCharacter` OtherActor)
  (set `self.InBox` false))

(event `/Game/PracticalWork38/Meta/Blueprints/BPI_Switchable.Light_On`
  (bind _output_get (set `self.IsOn` true))
  (`self.OnPressed` _output_get))

(event `/Game/PracticalWork38/Meta/Blueprints/BPI_Switchable.Light_Off`
  (bind _output_get (set `self.IsOn` false))
  (`self.OnPressed` _output_get))

(fn `UserConstructionScript`)