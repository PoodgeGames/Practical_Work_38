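; BP_Light is a light fixture that switches on and off in response to a press event from its Bind component.
; BeginPlay binds OnOffLight to that event, and its OnOff flag selects LightOff when true and LightOn when false.
; Each state sets the static mesh's Emissive_Val material parameter and toggles RectLight visibility, keeping the visible glow and emitted light in step.
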(event `self.ReceiveBeginPlay`
  (add `/Game/Blueprints/BP_Button.OnPressed` (`self.Bind`) (delegate `OnOffLight`)))

(event `OnOffLight`
  (params (OnOff :type Boolean))
  (if OnOff
    (`self.Light_Off`)
    (else
      (`self.Light_On`))))

(event `self.Light_On`
  (`MeshComponent.SetScalarParameterValueOnMaterials` (`self.StaticMesh`) "Emissive_Val" 100.0)
  (`SceneComponent.SetVisibility` (`self.RectLight`) true false))

(event `self.Light_Off`
  (`MeshComponent.SetScalarParameterValueOnMaterials` (`self.StaticMesh`) "Emissive_Val" 0.0)
  (`SceneComponent.SetVisibility` (`self.RectLight`) false false))

(fn `UserConstructionScript`)